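; Volumetric storm cloud actor for a DLC17 chapter that drives lightning positions in the cloud material through the MPCCloud parameter collection.
; Construction sets the storm center, moves the Niagara Flash component there with its scale, and seeds three fixed light locations.
; On BeginPlay, a looping timer randomizes the light locations with short random delays, the third reusing the second's coordinates.
; Flash stays put at runtime, as its reposition and spawn nodes are unconnected.
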(event Custom|StrickLighting
  (Variables|Default|Setfloatx (+ (* (Math|Random|RandomFloat) 2e+01) 5.0))
  (Variables|Default|Setfloaty (+ (* (Math|Random|RandomFloat) 5e+01) 5.0))
  (Rendering|Material|SetVectorParameterValue (Variables|Default|GetMPC_Cloud) (Variables|Default|GetLightLocation1) (Utilities|Struct|MakeLinearColor (Variables|Default|Getfloatx) (Variables|Default|Getfloaty) 0.0 0.0) :!class /Script/Engine.KismetMaterialLibrary)
  (Utilities|FlowControl|Delay (Math|Random|RandomFloat))
  (Variables|Default|Setfloatx (+ (* (Math|Random|RandomFloat) 2e+01) 5.0))
  (Variables|Default|Setfloaty (+ (* (Math|Random|RandomFloat) 5e+01) 5.0))
  (Rendering|Material|SetVectorParameterValue (Variables|Default|GetMPC_Cloud) (Variables|Default|GetLightLocation2) (Utilities|Struct|MakeLinearColor (Variables|Default|Getfloatx) (Variables|Default|Getfloaty) 0.0 0.0) :!class /Script/Engine.KismetMaterialLibrary)
  (Utilities|FlowControl|Delay (Math|Random|RandomFloat))
  (Rendering|Material|SetVectorParameterValue (Variables|Default|GetMPC_Cloud) (Variables|Default|GetLightLocation3) (Utilities|Struct|MakeLinearColor (Variables|Default|Getfloatx) (Variables|Default|Getfloaty) 0.0 0.0) :!class /Script/Engine.KismetMaterialLibrary))

(event EventBeginPlay
  (Utilities|Time|SetTimerbyEvent (delegate Custom|StrickLighting) (* (Variables|Default|GetLightMoveTime) 3.141592) true))

(event Collision|EventActorBeginOverlap
  (params (OtherActor :type Actor%20Object%20Reference)))

(event EventTick
  (params (DeltaSeconds :type Float%20%28single-precision%29)))

(fn ConstructionScript
  (CallFunction|ParameterSet)
  (Rendering|Material|SetVectorParameterValue (Variables|Default|GetMPC_Cloud) (Variables|Default|GetLightLocation1) (Utilities|Struct|MakeLinearColor 18.37 32.15 0.0 0.0) :!class /Script/Engine.KismetMaterialLibrary)
  (Rendering|Material|SetVectorParameterValue (Variables|Default|GetMPC_Cloud) (Variables|Default|GetLightLocation2) (Utilities|Struct|MakeLinearColor 9.84 48.62 0.0 0.0) :!class /Script/Engine.KismetMaterialLibrary)
  (Rendering|Material|SetVectorParameterValue (Variables|Default|GetMPC_Cloud) (Variables|Default|GetLightLocation3) (Utilities|Struct|MakeLinearColor 22.05 12.93 0.0 0.0) :!class /Script/Engine.KismetMaterialLibrary))

(fn ParameterSet
  (bind _stormcenterlocation (Variables|Default|GetStormCenterLocation))
  (bind (_r _g) (Math|Color|BreakColor _stormcenterlocation))
  (Niagara|SetNiagaraVariable(Float) (Variables|Default|GetFlash) "User.FlashScale" (Variables|Default|GetFlashScale))
  (Rendering|Material|SetVectorParameterValue (Variables|Default|GetMPC_Cloud) (LocalVariables|GetStormCenter) _stormcenterlocation :!class /Script/Engine.KismetMaterialLibrary)
  (Transformation|SetWorldLocation (Variables|Default|GetFlash) (Math|Vector|MakeVector (* _r 1e+05) (* _g 1e+05) (Variables|Default|GetHeight)) false false)
  (Rendering|Material|SetVectorParameterValue (Variables|Default|GetMPC_Cloud) (Variables|Default|GetLightLocation1) _stormcenterlocation :!class /Script/Engine.KismetMaterialLibrary))